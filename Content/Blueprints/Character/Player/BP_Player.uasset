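; BP_Player is the side-scrolling platformer player character, moving along world X with Enhanced Input and turning to face its travel direction.
; Jumps gain forgiveness from a retriggerable-delay input buffer checked on Tick and coyote time through a CanJumpInternal override.
; While falling, a downward foot trace makes the capsule block the platform channel.
; Landing on a BP_NPC defeats it and bounces; other NPC contact defeats the player, removing input and detaching the camera.
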(event `self.ReceiveBeginPlay`
  (`parent.ReceiveBeginPlay`)
  (bind _asplayer_controller (cast `PlayerController` (`self.GetController`)))
  (`EnhancedInputSubsystemInterface.AddMappingContext` (pcsubsystem `EnhancedInputLocalPlayerSubsystem` _asplayer_controller) "/Game/Input/IMC_Platformer.IMC_Platformer" 0 (struct)))

(event `self.ReceiveTick`
  (params (DeltaSeconds :type "Float (single-precision)"))
  (`parent.ReceiveTick` DeltaSeconds)
  (`self.Updatecontroller Rotation`)
  (`self.TraceForPlatform`)
  (if (and (`self.IsJumpBuferr`) (`self.CanJump`))
    (`self.Jump`)))

(event `EnhancedInput|/Game/Input/Actions/IA_Jump`
  (params (ActionValue :type Boolean) (ElapsedSeconds :type "Float (double-precision)") (TriggeredSeconds :type "Float (double-precision)") (InputAction :type "InputAction Object Reference" :default "/Game/Input/Actions/IA_Jump.IA_Jump"))
  (:`Started`
    (if (`self.CanJump`)
      (`self.Jump`)
      (else
        (set `self.IsJumpBuferr` true)
        (`KismetSystemLibrary.RetriggerableDelay` (`self.JumpBufferRange`))
        (set `self.IsJumpBuferr` false))))
  (:`Completed`
    (`self.StopJumping`)))

(event `EnhancedInput|/Game/Input/Actions/IA_Move`
  (params (ActionValue :type "Float (double-precision)") (ElapsedSeconds :type "Float (double-precision)") (TriggeredSeconds :type "Float (double-precision)") (InputAction :type "InputAction Object Reference" :default "/Game/Input/Actions/IA_Move.IA_Move"))
  (:`Triggered`
    (`self.AddMovementInput` (1.0 0.0 0.0) ActionValue)))

(event `self.CapsuleComponent.OnComponentBeginOverlap`
  (params (OverlappedComponent :type "PrimitiveComponent Object Reference") (OtherActor :type "Actor Object Reference") (OtherComp :type "PrimitiveComponent Object Reference") (OtherBodyIndex :type Integer) (bFromSweep :type Boolean) (SweepResult :type "HitResult Structure (by ref)"))
  (bind (_returnvalue_x _returnvalue_y _returnvalue_z) (`KismetMathLibrary.BreakVector` (`self.GetVelocity`)))
  (bind _asbp_npc (cast `/Game/Blueprints/Character/NPC/BP_NPC` OtherActor))
  (if (and (`NavMovementComponent.IsFalling` (`self.CharacterMovement`)) (< _returnvalue_z 0.0))
    (`self.Defeat` _asbp_npc)
    (`self.LaunchCharacter` (`KismetMathLibrary.MakeVector` 0.0 0.0 (`self.EnemyBounchLaunch`)) false true)
    (else
      (`self.Defeat`))))

(event `self.Defeat`
  (`parent.Defeat`)
  (bind _asplayer_controller (cast `PlayerController` (`self.GetController`)))
  (`EnhancedInputSubsystemInterface.RemoveMappingContext` (pcsubsystem `EnhancedInputLocalPlayerSubsystem` _asplayer_controller) "/Game/Input/IMC_Platformer.IMC_Platformer" (struct))
  (`SceneComponent.K2_DetachFromComponent` (`self.SpringArm`) "KeepWorld" "KeepRelative" "KeepRelative" true)
  (`GameplayStatics.PlaySound2D` "/Game/Sound/PlayerDefeated/S_PlayerDefeated_Cue.S_PlayerDefeated_Cue" 1.0 1.0 0.0 null null)
  (`GameplayStatics.PlayWorldCameraShake` "/Game/CameraShake/CS_Defeated.CS_Defeated_C" (`self.K2_GetActorLocation`) 0.0 1000.0 0.0))

(event `self.OnWalkingOffLedge`
  (params (PreviousFloorImpactNormal :type "Vector Structure (by ref)") (PreviousFloorContactNormal :type "Vector Structure (by ref)") (PreviousLocation :type "Vector Structure (by ref)") (TimeDelta :type "Float (single-precision)"))
  (set `self.IsIncoyotetime` true)
  (`KismetSystemLibrary.RetriggerableDelay` (`self.CoyoteTimeDelay`))
  (set `self.IsIncoyotetime` false))

(fn `CanJumpInternal`
  (returns (ReturnValue :type Boolean))
  (bind _returnvalue (`parent.CanJumpInternal`))
  (return (or _returnvalue (`self.IsIncoyotetime`))))

(fn `TraceForPlatform`
  (bind (_returnvalue_x _returnvalue_y _returnvalue_z) (`KismetMathLibrary.BreakVector` (`self.GetVelocity`)))
  (bind _returnvalue (`SceneComponent.K2_GetComponentLocation` (`self.FootPosition`)))
  (if (`NavMovementComponent.IsFalling` (`self.CharacterMovement`))
    (bind (_outhit _returnvalue_2) (`KismetSystemLibrary.LineTraceSingleForObjects` _returnvalue (+ _returnvalue (* (`KismetMathLibrary.Vector_Down`) (`self.PlatformCheckDistance`))) (`|MakeArray` "ObjectTypeQuery7" :!type "EObjectTypeQuery Enum")))
    (if (and _returnvalue_2 (< _returnvalue_z 0.0))
      (`PrimitiveComponent.SetCollisionResponseToChannel` (`self.CapsuleComponent`) "ECC_GameTraceChannel1" "ECR_Block"))))

(fn `Updatecontroller Rotation`
  (bind _returnvalue (`self.GetController`))
  (bind _returnvalue_2 (`self.GetController`))
  (bind _velocity_x (`KismetMathLibrary.BreakVector` (`MovementComponent.Velocity` (`self.CharacterMovement`))))
  (`/Engine/EditorBlueprintResources/StandardMacros.CompareFloat` _velocity_x
    (:`>`
      (`/Engine/EditorBlueprintResources/StandardMacros.IsValid` _returnvalue_2
        (:`Is Valid`
          (`Controller.SetControlRotation` _returnvalue_2 (`KismetMathLibrary.MakeRotator` 0.0)))))
    (:`<`
      (`/Engine/EditorBlueprintResources/StandardMacros.IsValid` _returnvalue
        (:`Is Valid`
          (`Controller.SetControlRotation` _returnvalue (`KismetMathLibrary.MakeRotator` 0.0 0.0 180.0)))))))

(fn `UserConstructionScript`
  (`parent.UserConstructionScript`))