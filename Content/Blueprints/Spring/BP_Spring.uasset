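; BP_Spring is a 2D platformer spring that launches the player character upward on contact.
; When BP_platformerchar overlaps the CharacterCheck component, it is launched along the up vector by LaunchPower, overriding vertical velocity but keeping horizontal motion.
; The PaperFlipbook then plays the active spring animation once without looping and swaps back to the idle flipbook when it finishes.
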(event `self.CharacterCheck.OnComponentBeginOverlap`
  (params (OverlappedComponent :type "PrimitiveComponent Object Reference") (OtherActor :type "Actor Object Reference") (OtherComp :type "PrimitiveComponent Object Reference") (OtherBodyIndex :type Integer) (bFromSweep :type Boolean) (SweepResult :type "HitResult Structure (by ref)"))
  (bind _asbp_platformerchar (cast `/Game/Blueprints/Character/BP_platformerchar` OtherActor))
  (`Character.LaunchCharacter` _asbp_platformerchar (* (`KismetMathLibrary.Vector_Up`) (`self.LaunchPower`)) false true)
  (`PaperFlipbookComponent.SetLooping` (`self.PaperFlipbook`) false)
  (`PaperFlipbookComponent.SetFlipbook` (`self.PaperFlipbook`) "/Game/PaperAssets/Spring/Spring__Active.Spring__Active")
  (`PaperFlipbookComponent.Play` (`self.PaperFlipbook`)))

(event `self.PaperFlipbook.OnFinishedPlaying`
  (`PaperFlipbookComponent.SetFlipbook` (`self.PaperFlipbook`) "/Game/PaperAssets/Spring/Spring__Idle_PNG_Flipbook.Spring__Idle_PNG_Flipbook"))

(fn `UserConstructionScript`)